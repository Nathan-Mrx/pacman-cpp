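; Pinky, the pink Pac-Man ghost, which feeds blackboard keys for its AI to ambush the player.
; A looping timer asks Pac-Man for his direction, and the callback targets a point offset ahead of him.
; Flee events toggle the scared state and sprite, while hitbox overlap kills Pac-Man or, under a power pellet, turns Pinky into dead eyes.
; Range overlap briefly flags AtRange, and BeginPlay records the spawn location after a delay.
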(event `self.hitbox.OnComponentBeginOverlap`
  (params (OverlappedComponent :type "PrimitiveComponent Object Reference") (OtherActor :type "Actor Object Reference") (OtherComp :type "PrimitiveComponent Object Reference") (OtherBodyIndex :type Integer) (bFromSweep :type Boolean) (SweepResult :type "HitResult Structure (by ref)"))
  (bind _asbp_pc_pac_man_character (cast `/Game/Pacman/Blueprints/BP_PC_PacManCharacter` OtherActor))
  (if (`/Game/Pacman/Blueprints/BP_PC_PacManCharacter.IsUnderPowerPelletEffect` _asbp_pc_pac_man_character)
    (`PaperSpriteComponent.SetSprite` (`self.PaperSprite`) "/Game/assets/ghosts/eyes_Sprite.eyes_Sprite")
    (`BlackboardComponent.SetValueAsBool` (`AIBlueprintHelperLibrary.GetBlackboard` null) "IsDead" true)
    (`GameplayStatics.PlaySound2D` "/Game/assets/sfx/pacman_eatghost.pacman_eatghost" 1.0 1.0 0.0 null null)
    (else
      (`/Game/Pacman/Blueprints/BP_PC_PacManCharacter.Die` _asbp_pc_pac_man_character))))

(event `Flee`
  (`PaperSpriteComponent.SetSprite` (`self.PaperSprite`) "/Game/assets/ghosts/blue_ghost_Sprite.blue_ghost_Sprite")
  (`BlackboardComponent.SetValueAsBool` (`AIBlueprintHelperLibrary.GetBlackboard` null) "IsScared" true))

(event `EndFlee`
  (`PaperSpriteComponent.SetSprite` (`self.PaperSprite`) "/Game/assets/ghosts/pinky_Sprite.pinky_Sprite")
  (`BlackboardComponent.SetValueAsBool` (`AIBlueprintHelperLibrary.GetBlackboard` null) "IsScared" false))

(event `self.ReceiveBeginPlay`
  (`KismetSystemLibrary.K2_SetTimerDelegate` (delegate `AskPacmanForDirection`) 0.5 true false 4.0)
  (`KismetSystemLibrary.Delay` 4.5)
  (`BlackboardComponent.SetValueAsVector` (`AIBlueprintHelperLibrary.GetBlackboard` null) "SpawnLocation" (`self.K2_GetActorLocation`)))

(event `AskPacmanForDirection`
  (bind _asbp_pc_pac_man_character (cast `/Game/Pacman/Blueprints/BP_PC_PacManCharacter` (`GameplayStatics.GetPlayerCharacter` 0)))
  (`/Game/Pacman/Blueprints/BP_PC_PacManCharacter.GivePinkyDirection` _asbp_pc_pac_man_character))

(event `GetPacmanDirection`
  (params (direction :type String :default "r"))
  (bind _returnvalue (`self.K2_GetActorLocation` (`GameplayStatics.GetPlayerCharacter` 0)))
  (`KismetSystemLibrary.PrintString` direction)
  (switch `string` direction
    (:`Default`
      (set `self.TargetLocation` _returnvalue))
    (:`r`
      (set `self.TargetLocation` (+ _returnvalue (300.0 0.0 0.0))))
    (:`l`
      (set `self.TargetLocation` (+ _returnvalue (-300.0 0.0 0.0))))
    (:`u`
      (set `self.TargetLocation` (+ _returnvalue (0.0 -300.0 0.0))))
    (:`b`
      (set `self.TargetLocation` (+ _returnvalue (0.0 300.0 0.0)))))
  (`BlackboardComponent.SetValueAsVector` (`AIBlueprintHelperLibrary.GetBlackboard` null) "TargetLocation" (`self.TargetLocation`)))

(event `self.Range.OnComponentBeginOverlap`
  (params (OverlappedComponent :type "PrimitiveComponent Object Reference") (OtherActor :type "Actor Object Reference") (OtherComp :type "PrimitiveComponent Object Reference") (OtherBodyIndex :type Integer) (bFromSweep :type Boolean) (SweepResult :type "HitResult Structure (by ref)"))
  (cast `/Game/Pacman/Blueprints/BP_PC_PacManCharacter` OtherActor)
  (`BlackboardComponent.SetValueAsBool` (`AIBlueprintHelperLibrary.GetBlackboard` null) "AtRange" true)
  (`KismetSystemLibrary.Delay` 3.0)
  (`BlackboardComponent.SetValueAsBool` (`AIBlueprintHelperLibrary.GetBlackboard` null) "AtRange" false))

(fn `UserConstructionScript`
  (`parent.UserConstructionScript`))