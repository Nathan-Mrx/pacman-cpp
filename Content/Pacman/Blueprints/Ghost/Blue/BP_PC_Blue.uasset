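; Blue ghost Inky for the Pac-Man game, whose behavior is fed through AI blackboard keys.
; A looping timer asks Pac-Man to give Blinky's location, and GetTargetLocation mirrors that position through Pac-Man in XY to set the target.
; Flee and EndFlee toggle the scared sprite and key.
; Overlapping Pac-Man kills him, or under power pellet effect turns Inky into eyes and flags it dead.
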(event `self.ReceiveActorBeginOverlap`
  (params (OtherActor :type "Actor Object Reference"))
  (bind _asbp_pc_pac_man_character (cast `/Game/Pacman/Blueprints/BP_PC_PacManCharacter` OtherActor))
  (if (`/Game/Pacman/Blueprints/BP_PC_PacManCharacter.IsUnderPowerPelletEffect` _asbp_pc_pac_man_character)
    (`PaperSpriteComponent.SetSprite` (`self.PaperSprite`) "/Game/assets/ghosts/eyes_Sprite.eyes_Sprite")
    (`BlackboardComponent.SetValueAsBool` (`AIBlueprintHelperLibrary.GetBlackboard` null) "IsDead" true)
    (`GameplayStatics.PlaySound2D` "/Game/assets/sfx/pacman_eatghost.pacman_eatghost" 1.0 1.0 0.0 null null)
    (else
      (`/Game/Pacman/Blueprints/BP_PC_PacManCharacter.Die` _asbp_pc_pac_man_character))))

(event `Flee`
  (`PaperSpriteComponent.SetSprite` (`self.PaperSprite`) "/Game/assets/ghosts/blue_ghost_Sprite.blue_ghost_Sprite")
  (`BlackboardComponent.SetValueAsBool` (`AIBlueprintHelperLibrary.GetBlackboard` null) "IsScared" true))

(event `GetTargetLocation`
  (params (BlinkyLocation :type "Vector Structure"))
  (bind _returnvalue (`self.K2_GetActorLocation` (`GameplayStatics.GetPlayerCharacter` 0)))
  (`BlackboardComponent.SetValueAsVector` (`AIBlueprintHelperLibrary.GetBlackboard` null) "TargetLocation" (+ (* (- BlinkyLocation _returnvalue) (-1.0 -1.0 1.0)) _returnvalue)))

(event `EndFlee`
  (`PaperSpriteComponent.SetSprite` (`self.PaperSprite`) "/Game/assets/ghosts/inky_Sprite.inky_Sprite")
  (`BlackboardComponent.SetValueAsBool` (`AIBlueprintHelperLibrary.GetBlackboard` null) "IsScared" false))

(event `self.ReceiveBeginPlay`
  (`KismetSystemLibrary.K2_SetTimerDelegate` (delegate `AskPacmanForLocation`) 0.5 true false 4.0)
  (`KismetSystemLibrary.Delay` 4.5)
  (`BlackboardComponent.SetValueAsVector` (`AIBlueprintHelperLibrary.GetBlackboard` null) "SpawnLocation" (`self.K2_GetActorLocation`)))

(event `AskPacmanForLocation`
  (bind _asbp_pc_pac_man_character (cast `/Game/Pacman/Blueprints/BP_PC_PacManCharacter` (`GameplayStatics.GetPlayerCharacter` 0)))
  (`/Game/Pacman/Blueprints/BP_PC_PacManCharacter.GiveBlinkyLocationToInky` _asbp_pc_pac_man_character))

(fn `UserConstructionScript`
  (`parent.UserConstructionScript`))