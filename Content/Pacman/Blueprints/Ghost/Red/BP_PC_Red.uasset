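; Blueprint for the red Pac-Man ghost (Blinky), which drives its AI through blackboard keys and mirrors its state with sprite swaps.
; BeginPlay stores the spawn location on the blackboard.
; Flee and EndFlee toggle IsScared, switching between the blue and Blinky sprites.
; Overlapping Pac-Man during a power pellet effect shows the eyes sprite and sets IsDead; this file never clears that flag.
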(event `self.ReceiveActorBeginOverlap`
  (params (OtherActor :type "Actor Object Reference"))
  (bind _asbp_pc_pac_man_character (cast `/Game/Pacman/Blueprints/BP_PC_PacManCharacter` OtherActor))
  (if (`/Game/Pacman/Blueprints/BP_PC_PacManCharacter.IsUnderPowerPelletEffect` _asbp_pc_pac_man_character)
    (`PaperSpriteComponent.SetSprite` (`self.PaperSprite`) "/Game/assets/ghosts/eyes_Sprite.eyes_Sprite")
    (`BlackboardComponent.SetValueAsBool` (`AIBlueprintHelperLibrary.GetBlackboard` null) "IsDead" true)))

(event `Flee`
  (`PaperSpriteComponent.SetSprite` (`self.PaperSprite`) "/Game/assets/ghosts/blue_ghost_Sprite.blue_ghost_Sprite")
  (`BlackboardComponent.SetValueAsBool` (`AIBlueprintHelperLibrary.GetBlackboard` null) "IsScared" true))

(event `EndFlee`
  (`PaperSpriteComponent.SetSprite` (`self.PaperSprite`) "/Game/assets/ghosts/blinky_Sprite.blinky_Sprite")
  (`BlackboardComponent.SetValueAsBool` (`AIBlueprintHelperLibrary.GetBlackboard` null) "IsScared" false))

(event `self.ReceiveBeginPlay`
  (`BlackboardComponent.SetValueAsVector` (`AIBlueprintHelperLibrary.GetBlackboard` null) "SpawnLocation" (`self.K2_GetActorLocation`)))

(fn `UserConstructionScript`
  (`parent.UserConstructionScript`))